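; HUD Blueprint that shows the score, player level and game-over prompt for the guide game.
; On BeginPlay it casts the game mode to BP_Guide_GameMode and caches it.
; Each DrawHUD call reads Score, Level and GameOver from that game mode and draws them as scaled canvas text, adding red GAME OVER and Press Enter lines when the game ends.
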(event EventBeginPlay
  (bind _asbp_guide_game_mode (Utilities|Casting|CastToBP_Guide_GameMode (Game|GetGameMode)))
  (Variables|Default|SetMy_Guide_GameMode _asbp_guide_game_mode))

(event EventDrawHUD
  (params (SizeX :type Integer) (SizeY :type Integer))
  (HUD|DrawText (Utilities|String|BuildString(Integer) "Score: " "" (Variables|/Game/BPGuide/BP_Guide_GameMode.BP_Guide_GameMode_C|GetScore (Variables|Default|GetMy_Guide_GameMode))) "(R=0,G=0,B=0,A=1)" 3e+02 1e+01 0 3.0 false)
  (HUD|DrawText (Utilities|String|BuildString(Integer) "Player Level: " "" (Variables|/Game/BPGuide/BP_Guide_GameMode.BP_Guide_GameMode_C|GetLevel (Variables|Default|GetMy_Guide_GameMode))) "(R=0,G=0,B=0,A=1)" 0.0 0.0 0 3.0 false)
  (if (Variables|/Game/BPGuide/BP_Guide_GameMode.BP_Guide_GameMode_C|GetGameOver (Variables|Default|GetMy_Guide_GameMode))
    (HUD|DrawText "GAME OVER" "(R=1.000000,G=0.126759,B=0.037092,A=1.000000)" 4e+02 2e+02 0 3.0 false)
    (HUD|DrawText "Press Enter" "(R=1.000000,G=0.013544,B=0.000000,A=1.000000)" 4e+02 4e+02 0 3.0 false)))

(fn ConstructionScript)